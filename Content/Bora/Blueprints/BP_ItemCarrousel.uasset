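; BP_ItemCarrousel is an actor that manages four item spawner child actors, filling them with randomly chosen minigame items.
; At begin play it registers each spawner with a slot index and staggers its up-down motion.
; Starting the spawn loop loads games and weights from DT_Minigames, then fills every slot by weighted random selection.
; SpawnNewItem refills a single slot using the same weighted pick, which allows duplicates.
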(event Custom|StartItemSpawnLoop
  (CallFunction|FillGamesArray)
  (for _index (range 0 3)
    (bind _decidedgame (CallFunction|DecideGame))
    (Default|SpawnItem (Utilities|Array|Get(acopy) (Variables|Default|GetItemSpawnerArray) _index) _decidedgame)))

(event Custom|SpawnNewItem
  (params (Spawn%20Slot :type Integer))
  (bind _decidedgame (CallFunction|DecideGame))
  (Default|SpawnItem (Utilities|Array|Get(acopy) (Variables|Default|GetItemSpawnerArray) Spawn%20Slot) _decidedgame))

(event EventBeginPlay
  (bind _asgm_xrgame_mode (Utilities|Casting|CastToGM_XRGameMode (Game|GetGameMode)))
  (Variables|Default|SetGMRef _asgm_xrgame_mode)
  (for (_array_element _array_index) (Utilities|Array|MakeArray (Variables|Default|GetBP_ItemSpawner1) (Variables|Default|GetBP_ItemSpawner2) (Variables|Default|GetBP_ItemSpawner3) (Variables|Default|GetBP_ItemSpawner4))
    (bind _asbp_item_spawner (Utilities|Casting|CastToBP_ItemSpawner (Variables|/Script/Engine.ChildActorComponent|GetChildActor _array_element)))
    (Utilities|Array|Add (Variables|Default|GetItemSpawnerArray) _asbp_item_spawner)
    (Variables|/Game/Bora/Blueprints/BP_ItemSpawner.BP_ItemSpawner_C|SetSpawnerSlot _asbp_item_spawner _array_index)
    (Default|StartUpDown _asbp_item_spawner (* _array_index 0.5))))

(fn ConstructionScript)

(fn DecideGame
  (LocalVariables|SetRandomFloat (Math|Random|RandomFloatinRange 0.0 (Variables|Default|GetCombinedWeights)))
  (bind (_array_element _array_index) (Utilities|Array|ForEachLoopwithBreak (Variables|Default|GetGameWeights) :!label _label)
    (:LoopBody
      (LocalVariables|SetCurrentIndex _array_index)
      (bind _output_get (LocalVariables|SetRandomFloat (Math|Float|Max(Float) (- (LocalVariables|GetRandomFloat) _array_element) 0.0)))
      (if (== _output_get 0.0)
        (goto _label Break)))
    (:Completed
      (return (.Blueprint (Utilities|Struct|BreakST_Minigame (Utilities|Array|Get(acopy) (Variables|Default|GetGames) (LocalVariables|GetCurrentIndex))))))))

(fn FillGamesArray
  (bind _outrownames (DataTable|GetDataTableRowNames "/Game/Bora/Blueprints/DT_Minigames.DT_Minigames"))
  (for _array_element _outrownames
    (bind _returnvalue (Utilities|GetDataTableRow "/Game/Bora/Blueprints/DT_Minigames.DT_Minigames" _array_element)
      (:then
        (Utilities|Array|Add (Variables|Default|GetGames) _returnvalue)
        (Utilities|Array|Add (Variables|Default|GetGameWeights) (.Weight (Utilities|Struct|BreakST_Minigame _returnvalue)))
        (LocalVariables|SetRunningWeight (+ (LocalVariables|GetRunningWeight) (.Weight (Utilities|Struct|BreakST_Minigame _returnvalue)))))))
  (Variables|Default|SetCombinedWeights (LocalVariables|GetRunningWeight)))