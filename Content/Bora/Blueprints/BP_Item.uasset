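; BP_Item is a grabbable VR minigame item that adds or deducts grand timer time when destroyed.
; It reads its reward and penalty from DT_Minigames by ItemName.
; Grabbing starts an expiry timer that fails the item unless dropped, and the first grab notifies the GameMode with its spawn slot.
; It toggles hand messages through the motion controller's owner, avoiding a hard VR pawn reference.
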(event OnGrabbed(BP_GrabComponent)
  (bind _bp_grabcomponent (Variables|Default|GetBP_GrabComponent))
  (Class|BPIPawnAnim|HideUnhideHand(Message) (Components|GetOwner (Variables|/Game/XRFramework/Blueprints/BP_GrabComponent.BP_GrabComponent_C|GetMotionControllerRef _bp_grabcomponent)) true (Utilities|Enum|Equal(Enum) (Default|GetHeldbyHand _bp_grabcomponent) "Right"))
  (bind _returnvalue (Utilities|Time|SetTimerbyEvent (delegate Custom|Expiry) (Variables|Default|GetExpiryTime)))
  (Variables|Default|SetTimerHandle _returnvalue)
  (CallFunction|InformGMonGrab))

(event OnDropped(BP_GrabComponent)
  (bind _bp_grabcomponent (Variables|Default|GetBP_GrabComponent))
  (Class|BPIPawnAnim|HideUnhideHand(Message) (Components|GetOwner (Variables|/Game/XRFramework/Blueprints/BP_GrabComponent.BP_GrabComponent_C|GetMotionControllerRef _bp_grabcomponent)) false (Utilities|Enum|Equal(Enum) (Default|GetHeldbyHand _bp_grabcomponent) "Right"))
  (if (Utilities|Time|IsValidTimerHandle (Variables|Default|GetTimerHandle))
    (Utilities|Time|ClearandInvalidateTimerbyHandle (Variables|Default|GetTimerHandle))))

(event Custom|InformGMOnGrab
  ;[0.15 0.15 0.15 0.5] To Spawn New Item
  (Utilities|FlowControl|DoOnce false
    (:Completed
      (Default|OnItemGrabbed (Variables|Default|GetGMRef) (Variables|Default|GetSpawnSlot)))))

(event Custom|DestroyItem
  (params (Success? :type Boolean))
  (bind _gmref (Variables|Default|GetGMRef))
  ;[0.15 0.15 0.15 0.5] Destroy
  (if Success?
    (Default|AddtoGrandTimer _gmref (Variables|Default|GetSuccessReward))
    (else
      (Default|AddtoGrandTimer _gmref (* (Variables|Default|GetFailPenalty) -1.0))))
  (Actor|DestroyActor))

(event Custom|Expiry
  (CallFunction|DestroyItem false))

(event Custom|Grabbed
  ;[0.15 0 0 0.5] Test
  (bind _returnvalue (Utilities|Time|SetTimerbyEvent (delegate Custom|Expiry) (Variables|Default|GetExpiryTime)))
  (Variables|Default|SetTimerHandle _returnvalue)
  (CallFunction|InformGMonGrab))

(event Custom|Released
  ;[0.15 0 0 0.5] Test
  (if (Utilities|Time|IsValidTimerHandle (Variables|Default|GetTimerHandle))
    (Utilities|Time|ClearandInvalidateTimerbyHandle (Variables|Default|GetTimerHandle))))

(event EventBeginPlay
  (bind _asgm_xrgame_mode (Utilities|Casting|CastToGM_XRGameMode (Game|GetGameMode)))
  (Variables|Default|SetGMRef _asgm_xrgame_mode)
  (bind _returnvalue (Utilities|GetDataTableRow "/Game/Bora/Blueprints/DT_Minigames.DT_Minigames" (Variables|Default|GetItemName))
    (:then
      (Variables|Default|SetFailPenalty (.Penalty (Utilities|Struct|BreakST_Minigame _returnvalue)))
      (Variables|Default|SetSuccessReward (.Reward (Utilities|Struct|BreakST_Minigame _returnvalue))))))

(event EventDestroyed
  (bind _bp_grabcomponent (Variables|Default|GetBP_GrabComponent))
  (if (Variables|/Game/XRFramework/Blueprints/BP_GrabComponent.BP_GrabComponent_C|GetbIsHeld _bp_grabcomponent)
    (Class|BPIPawnAnim|HideUnhideHand(Message) (Components|GetOwner (Variables|/Game/XRFramework/Blueprints/BP_GrabComponent.BP_GrabComponent_C|GetMotionControllerRef _bp_grabcomponent)) false (Utilities|Enum|Equal(Enum) (Default|GetHeldbyHand _bp_grabcomponent) "Right"))))

(fn ConstructionScript)