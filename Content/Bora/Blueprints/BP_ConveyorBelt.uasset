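; Conveyor belt actor that scrolls alternating black and gray tiles and carries physics objects resting on it.
; The construction script builds upper and lower tile rows as instanced meshes; after a two-second startup delay, Tick loops only the upper instances using a modulo offset scaled by actor Y scale.
; A box overlap tracks simulating root components, whose world Y velocity Tick overrides from belt direction and speed.
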(event OnComponentBeginOverlap(Box)
  (params (OverlappedComponent :type Primitive%20Component%20Object%20Reference) (OtherActor :type Actor%20Object%20Reference) (OtherComp :type Primitive%20Component%20Object%20Reference) (OtherBodyIndex :type Integer) (bFromSweep :type Boolean) (SweepResult :type Hit%20Result%20Structure%20%28by%20ref%29))
  (bind _asprimitive_component (Utilities|Casting|CastToPrimitiveComponent (Variables|/Script/Engine.Actor|GetRootComponent OtherActor)))
  (if (Physics|IsSimulatingPhysics _asprimitive_component "None")
    (Utilities|Array|Add (Variables|Default|GetComponentsOnBelt) _asprimitive_component)))

(event OnComponentEndOverlap(Box)
  (params (OverlappedComponent :type Primitive%20Component%20Object%20Reference) (OtherActor :type Actor%20Object%20Reference) (OtherComp :type Primitive%20Component%20Object%20Reference) (OtherBodyIndex :type Integer))
  (bind _asprimitive_component (Utilities|Casting|CastToPrimitiveComponent (Variables|/Script/Engine.Actor|GetRootComponent OtherActor)))
  (Utilities|Array|RemoveItem (Variables|Default|GetComponentsOnBelt) _asprimitive_component))

(event EventBeginPlay
  (Utilities|FlowControl|Delay 2.0)
  (Variables|Default|SetShouldMove? true)
  (bind _output_get (Variables|Default|SetActorScale (.y (Transformation|GetActorScale3D))))
  (Variables|Default|SetEffectiveTileSpacing (* _output_get (Variables|Default|GetTileSpacing)))
  (Variables|Default|SetEffectiveLoopLength (* (Variables|Default|GetActorScale) (Variables|Default|GetLoopLength))))

(event EventTick
  (params (DeltaSeconds :type Float%20%28single-precision%29))
  (bind _uppertppoint (Variables|Default|GetUpperTpPoint))
  (bind _uppertppoint_2 (Variables|Default|GetUpperTpPoint))
  (bind _returnvalue (Transformation|GetWorldTransform _uppertppoint))
  (bind _returnvalue_2 (Transformation|GetWorldTransform _uppertppoint_2))
  (if (Variables|Default|GetShouldMove?)
    (Variables|Default|SetBeltOffset (Math|Float|%(Float) (+ (Variables|Default|GetBeltOffset) (* DeltaSeconds (Variables|Default|GetBeltSpeed))) (Variables|Default|GetEffectiveLoopLength)))
    ;[0.15 0.15 0.15 0.5] Move Black Tiles
    (for _index (range 0 (- (Components|InstancedStaticMesh|GetInstanceCount (Variables|Default|GetUpperBlackTiles)) 1))
      (Components|InstancedStaticMesh|UpdateInstanceTransform (Variables|Default|GetUpperBlackTiles) _index (Math|Transform|MakeTransform (+ (.location _returnvalue_2) (* (Math|Vector|GetRightVector _uppertppoint_2) -1.0 (Math|Float|%(Float) (+ (Variables|Default|GetBeltOffset) (* _index (Variables|Default|GetEffectiveTileSpacing) 2.0)) (Variables|Default|GetEffectiveLoopLength)))) (.rotation _returnvalue_2) (.scale _returnvalue_2)) true false true))
    ;[0.15 0.15 0.15 0.5] Move Gray Tiles
    (for _index_2 (range 0 (- (Components|InstancedStaticMesh|GetInstanceCount (Variables|Default|GetUpperGrayTiles)) 1))
      (Components|InstancedStaticMesh|UpdateInstanceTransform (Variables|Default|GetUpperGrayTiles) _index_2 (Math|Transform|MakeTransform (+ (.location _returnvalue) (* (Math|Vector|GetRightVector _uppertppoint) -1.0 (Math|Float|%(Float) (+ (Variables|Default|GetBeltOffset) (* _index_2 (Variables|Default|GetEffectiveTileSpacing) 2.0) (Variables|Default|GetEffectiveTileSpacing)) (Variables|Default|GetEffectiveLoopLength)))) (.rotation _returnvalue) (.scale _returnvalue)) true false true))
    ;[0.15 0.15 0.15 0.5] Move Actors
    (for _array_element (Variables|Default|GetComponentsOnBelt)
      (bind _returnvalue_3 (Physics|GetPhysicsLinearVelocity _array_element "None"))
      (Physics|SetPhysicsLinearVelocity _array_element (Math|Vector|MakeVector (.x _returnvalue_3) (.y (* (Math|Vector|GetRightVector (Variables|Default|GetFrame)) -1.0 (Variables|Default|GetBeltSpeed) (Variables|Default|GetSpeedMultiplierForItems))) (.z _returnvalue_3)) false "None"))))

(fn ConstructionScript
  ;[0.15 0.15 0.15 0.5] Clear Instances of Tiles
  (Components|InstancedStaticMesh|ClearInstances (Variables|Default|GetLowerBlackTiles))
  (Components|InstancedStaticMesh|ClearInstances (Variables|Default|GetLowerGrayTiles))
  (Components|InstancedStaticMesh|ClearInstances (Variables|Default|GetUpperBlackTiles))
  (Components|InstancedStaticMesh|ClearInstances (Variables|Default|GetUpperGrayTiles))
  ;[0.15 0.15 0.15 0.5] Construct Upper Belt
  (for _index (range 0 (- (Variables|Default|GetTileCount) 1))
    (if (== (Math|Integer|%(Integer) _index 2) 0)
      (Components|InstancedStaticMesh|AddInstance (Variables|Default|GetUpperBlackTiles) (Math|Transform|MakeTransform (+ (Variables|Default|GetUpperTileStartPoint) (* _index (* (Math|Vector|GetRightVector (Variables|Default|GetFrame)) -1.0) (Variables|Default|GetEffectiveTileSpacing))) "0, 0, 0" "1.000000,1.000000,1.000000") false)
      (else
        (Components|InstancedStaticMesh|AddInstance (Variables|Default|GetUpperGrayTiles) (Math|Transform|MakeTransform (+ (Variables|Default|GetUpperTileStartPoint) (* _index (* (Math|Vector|GetRightVector (Variables|Default|GetFrame)) -1.0) (Variables|Default|GetEffectiveTileSpacing))) "0, 0, 0" "1.000000,1.000000,1.000000") false))))
  ;[0.15 0.15 0.15 0.5] Construct Lower Belt
  (for _index_2 (range 0 (- (Variables|Default|GetTileCount) 1))
    (if (== (Math|Integer|%(Integer) _index_2 2) 0)
      (Components|InstancedStaticMesh|AddInstance (Variables|Default|GetLowerBlackTiles) (Math|Transform|MakeTransform (+ (* _index_2 (Math|Vector|GetRightVector (Variables|Default|GetFrame)) (Variables|Default|GetEffectiveTileSpacing)) (Variables|Default|GetLowerTileStartPoint)) "0, 0, 0" "1.000000,1.000000,1.000000") false)
      (else
        (Components|InstancedStaticMesh|AddInstance (Variables|Default|GetLowerGrayTiles) (Math|Transform|MakeTransform (+ (* _index_2 (Math|Vector|GetRightVector (Variables|Default|GetFrame)) (Variables|Default|GetEffectiveTileSpacing)) (Variables|Default|GetLowerTileStartPoint)) "0, 0, 0" "1.000000,1.000000,1.000000") false)))))