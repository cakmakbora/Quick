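; BP_ItemSpawner is an item spawner actor that spawns items onto a component that can bob vertically.
; SpawnItem waits briefly, spawns the given class at the Scene component's transform with a spawner slot, then attaches it to that component.
; StartUpDown waits a caller-supplied delay before running UpDown, whose timeline lerps the Scene component's height up to MaxHeight, carrying attached items along.
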(event Custom|SpawnItem
  (params (ItemToBeSpawned :type BP%20Item%20Class%20Reference))
  (Utilities|FlowControl|Delay 0.5)
  (bind _returnvalue (Game|SpawnActorfromClass ItemToBeSpawned (Transformation|GetWorldTransform (Variables|Default|GetScene)) "Undefined" "MultiplyWithRoot" 0 (Variables|Default|GetSpawnerSlot) 0))
  (Transformation|AttachComponentToComponent _returnvalue (Variables|Default|GetScene) "None" "KeepWorld" "KeepWorld" "KeepWorld" true))

(event Custom|UpDown
  (bind _progress (Timeline|Timeline Play)
    (:Update
      (Transformation|SetRelativeLocation (Variables|Default|GetScene) (Math|Vector|MakeVector 0.0 0.0 (Math|Float|Lerp 0.0 (Variables|Default|GetMaxHeight) _progress)) false false))))

(event Custom|StartUpDown
  (params (Delay :type Float%20%28double-precision%29))
  (Utilities|FlowControl|Delay Delay)
  (CallFunction|UpDown))

(fn ConstructionScript)