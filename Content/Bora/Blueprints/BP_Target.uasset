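; BP_Target is a hittable target that, while active, awards bonus time to the BP_ItemCarousel found at BeginPlay.
; Selected lights it with a neon material and starts a randomized timer that calls Deselect to darken and deactivate it.
; BulletHit or any hit on the Target component adds the bonus to the carousel's grand timer, deselects the target and clears the pending timer.
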(event OnComponentHit(Target)
  (params (HitComponent :type Primitive%20Component%20Object%20Reference) (OtherActor :type Actor%20Object%20Reference) (OtherComp :type Primitive%20Component%20Object%20Reference) (NormalImpulse :type Vector :default "0, 0, 0") (Hit :type Hit%20Result%20Structure%20%28by%20ref%29))
  (if (Variables|Default|GetisActive)
    (Default|AddtoGrandTimer (Variables|Default|GetCarousel) (Variables|Default|GetTimeBonus))
    (CallFunction|Deselect)
    (if (Utilities|Time|IsValidTimerHandle (Variables|Default|GetTimerHandle))
      (Utilities|Time|ClearandInvalidateTimerbyHandle (Variables|Default|GetTimerHandle)))))

(event Custom|Selected
  (Rendering|Material|SetMaterial (Variables|Default|GetTarget) 0 "/Game/Bora/Models/Target/MI_NeonColor.MI_NeonColor")
  (Variables|Default|SetisActive true)
  (bind _returnvalue (Utilities|Time|SetTimerbyEvent (delegate Custom|Deselect) (Math|Random|RandomFloatinRange (Variables|Default|GetMinActiveTime) (Variables|Default|GetMaxActiveTime))))
  (Variables|Default|SetTimerHandle _returnvalue))

(event Custom|Deselect
  (Rendering|Material|SetMaterial (Variables|Default|GetTarget) 0 "/Game/Bora/Models/Target/DarkParts.DarkParts")
  (Variables|Default|SetisActive false))

(event Custom|BulletHit
  (if (Variables|Default|GetisActive)
    (Default|AddtoGrandTimer (Variables|Default|GetCarousel) (Variables|Default|GetTimeBonus))
    (CallFunction|Deselect)
    (if (Utilities|Time|IsValidTimerHandle (Variables|Default|GetTimerHandle))
      (Utilities|Time|ClearandInvalidateTimerbyHandle (Variables|Default|GetTimerHandle)))))

(event EventBeginPlay
  (bind _returnvalue (Actor|GetActorOfClass "/Game/Bora/Blueprints/BP_ItemCarousel.BP_ItemCarousel_C"))
  (Variables|Default|SetCarousel _returnvalue))

(fn ConstructionScript)