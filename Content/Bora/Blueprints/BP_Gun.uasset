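; BP_Gun is a held pistol item with limited ammo that fires BP_Bullet projectiles.
; Trigger spends a round and spawns a bullet at the Muzzle transform, scaled by BulletScale, with the gun as owner and player pawn as instigator.
; BulletMiss increments ProjectilesHit and destroys the gun once that count equals the initial ammo count.
; A haptic fire effect for the holding hand is present but never runs.
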(event Custom|BulletMiss
  ;[0.15 0.15 0.15 0.5] Bullet Missed
  (bind _result (Math|Integer|IncrementInt (Variables|Default|GetProjectilesHit))
    (:%20%20
      (if (== _result (Variables|Default|GetInitialBulletCount))
        (CallFunction|DestroyItem false)))))

(event EventTrigger
  (bind _muzzle (Variables|Default|GetMuzzle))
  (if (> (Variables|Default|GetBulletCount) 0)
    (Math|Integer|DecrementInt (Variables|Default|GetBulletCount)
      (:%20%20
        (Game|SpawnActorfromClass "/Game/Bora/Blueprints/BP_Bullet.BP_Bullet_C" (Math|Transform|MakeTransform (Transformation|GetWorldLocation _muzzle) (Transformation|GetWorldRotation _muzzle) (* (Transformation|GetWorldScale _muzzle) (Variables|Default|GetBulletScale))) "Undefined" "OverrideRootScale" self (Game|Player|GetPlayerPawn 0))))))

(event EventBeginPlay
  (|CallParentFunction)
  (Variables|Default|SetBulletCount (Variables|Default|GetInitialBulletCount)))

(fn ConstructionScript)