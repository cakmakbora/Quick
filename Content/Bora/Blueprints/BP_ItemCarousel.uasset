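; Item carousel that spawns weighted-random minigame items in four slots and also manages a countdown timer and shooting targets.
; Minigame classes and weights come from DT_Minigames; grabbed slots refill after a delay.
; Tick drains GrandTimer, shown on a temporary test widget, and activates random small or big targets at random intervals up to a cap, balancing sizes.
; TargetCleanup returns targets to their pools, replenishing a size that runs out.
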(event Custom|AddToGrandTimer
  (params (AmountToBeAdded :type Float%20%28double-precision%29))
  ;[0.15 0.15 0.15 0.5] Add/Subtract Time
  (Variables|Default|SetGrandTimer (Math|Float|Max(Float) (+ (Variables|Default|GetGrandTimer) AmountToBeAdded) 0.0)))

(event Custom|StartItemSpawnLoop
  (CallFunction|FillGamesArray)
  (for (_ _array_index) (Variables|Default|GetItemSpawnerArray)
    (CallFunction|SpawnItem _array_index)))

(event Custom|OnItemGrabbed
  (params (Slot :type Integer))
  (Utilities|FlowControl|Delay (Variables|Default|GetItemSpawnDelay))
  (CallFunction|SpawnItem Slot))

(event EventBeginPlay
  (Variables|Default|SetItemSpawnerArray (Utilities|Array|MakeArray (Variables|Default|GetSpawn1) (Variables|Default|GetSpawn2) (Variables|Default|GetSpawn3) (Variables|Default|GetSpawn4)))
  ;[0.15 0 0 0.5] For Testing Purposes (Remove Later)
  (bind _returnvalue (UserInterface|CreateWidget "/Game/Bora/Blueprints/WBP_Test.WBP_Test_C" (Game|GetPlayerController 0)))
  (bind _output_get (Variables|Default|SetWBPRef _returnvalue))
  (UserInterface|Viewport|AddtoViewport _output_get 0)
  (bind _outactors (Actor|GetAllActorsOfClass "/Game/Bora/Blueprints/BP_SmallTarget.BP_SmallTarget_C"))
  (Variables|Default|SetSmallTargets _outactors)
  (bind _outactors_2 (Actor|GetAllActorsOfClass "/Game/Bora/Blueprints/BP_BigTarget.BP_BigTarget_C"))
  (Variables|Default|SetBigTargets _outactors_2)
  (CallFunction|ActivateTarget false)
  (CallFunction|ActivateTarget true)
  (Utilities|FlowControl|Delay 2.0)
  (CallFunction|StartItemSpawnLoop))

(event EventTick
  (params (DeltaSeconds :type Float%20%28single-precision%29))
  (Utilities|FlowControl|Sequence
    (:then_0
      (bind _output_get (Variables|Default|SetGrandTimer (Math|Float|Max(Float) (- (Variables|Default|GetGrandTimer) DeltaSeconds) 0.0)))
      ;[0.15 0 0 0.5] For Testing Purposes (Remove Later)
      (Default|UpdateGrandTimer (Variables|Default|GetWBPRef) (Math|Float|Truncate _output_get)))
    (:then_1
      ;[0.15 0.15 0.15 0.5] Activate Targets
      (Variables|Default|SetTargetActivatorTimer (+ (Variables|Default|GetTargetActivatorTimer) DeltaSeconds))
      (CallFunction|CheckforTargetActivation))))

(fn ConstructionScript)

(fn DecideGame
  (LocalVariables|SetRandomFloat (Math|Random|RandomFloatinRange 0.0 (Variables|Default|GetCombinedWeights)))
  (bind (_array_element _array_index) (Utilities|Array|ForEachLoopwithBreak (Variables|Default|GetGameWeights) :!label _label)
    (:LoopBody
      (LocalVariables|SetCurrentIndex _array_index)
      (bind _output_get (LocalVariables|SetRandomFloat (Math|Float|Max(Float) (- (LocalVariables|GetRandomFloat) _array_element) 0.0)))
      (if (== _output_get 0.0)
        (goto _label Break)))
    (:Completed
      (return (.Blueprint (Utilities|Struct|BreakST_Minigame (Utilities|Array|Get(acopy) (Variables|Default|GetGames) (LocalVariables|GetCurrentIndex))))))))

(fn FillGamesArray
  (bind _outrownames (DataTable|GetDataTableRowNames "/Game/Bora/Blueprints/DT_Minigames.DT_Minigames"))
  (for _array_element _outrownames
    (bind _returnvalue (Utilities|GetDataTableRow "/Game/Bora/Blueprints/DT_Minigames.DT_Minigames" _array_element)
      (:then
        (Utilities|Array|Add (Variables|Default|GetGames) _returnvalue)
        (Utilities|Array|Add (Variables|Default|GetGameWeights) (.Weight (Utilities|Struct|BreakST_Minigame _returnvalue)))
        (LocalVariables|SetRunningWeight (+ (LocalVariables|GetRunningWeight) (.Weight (Utilities|Struct|BreakST_Minigame _returnvalue)))))))
  (Variables|Default|SetCombinedWeights (LocalVariables|GetRunningWeight)))

(fn SpawnItem
  (params (SpawnSlot :type Integer))
  (bind _itemspawnerarray (Variables|Default|GetItemSpawnerArray))
  (bind _output (Utilities|Array|Get(acopy) _itemspawnerarray SpawnSlot))
  (bind _decidedgame (CallFunction|DecideGame))
  (bind _returnvalue (Game|SpawnActorfromClass _decidedgame (Transformation|GetWorldTransform _output) "Undefined" "MultiplyWithRoot" 0 SpawnSlot self 0))
  (Transformation|AttachComponentToComponent _returnvalue _output "None" "KeepWorld" "KeepWorld" "KeepWorld" true)
  (Collision|SetCollisionResponsetoChannel (Variables|/Game/Bora/Blueprints/BP_Item.BP_Item_C|GetRoot _returnvalue) "ECC_GameTraceChannel3" "ECR_Ignore"))

(fn ActivateTarget
  (params (Small? :type Boolean))
  (if Small?
    (bind _output_get (LocalVariables|SetSmallTarget (.OutItem (Utilities|Array|Random (Variables|Default|GetSmallTargets)))))
    (Utilities|Array|RemoveItem (Variables|Default|GetSmallTargets) _output_get)
    (Default|Selected (LocalVariables|GetSmallTarget))
    (Math|Integer|IncrementInt (Variables|Default|GetActiveSmallTargetCount)
      (:%20%20
        _))
    (else
      (bind _output_get_2 (LocalVariables|SetBigTarget (.OutItem (Utilities|Array|Random (Variables|Default|GetBigTargets)))))
      (Utilities|Array|RemoveItem (Variables|Default|GetBigTargets) _output_get_2)
      (Default|Selected (LocalVariables|GetBigTarget))
      (Math|Integer|IncrementInt (Variables|Default|GetActiveBigTargetCount)
        (:%20%20
          _))))
  (Variables|Default|SetTargetActivatorTimer 0.0)
  (Variables|Default|SetTargetActivationTime (Math|Random|RandomFloatinRange (Variables|Default|GetTargetTimerMin) (Variables|Default|GetTargetTimerMax))))

(fn CheckforTargetActivation
  ;[0.15 0.15 0.15 0.5] Is it time?
  (if (>= (Variables|Default|GetTargetActivatorTimer) (Variables|Default|GetTargetActivationTime))
    ;[0.15 0.15 0.15 0.5] Are we below max target count?
    (if (< (+ (Variables|Default|GetActiveSmallTargetCount) (Variables|Default|GetActiveBigTargetCount)) (Variables|Default|GetMaxActiveTargetCount))
      ;[0.15 0.15 0.15 0.5] Decision
      (if (Math|Random|RandomBool)
        (if (< (Variables|Default|GetActiveSmallTargetCount) (Utilities|CeilingDivision (Variables|Default|GetMaxActiveTargetCount) 2))
          (CallFunction|ActivateTarget true :!label _label)
          (else
            (CallFunction|ActivateTarget false :!label _label_2)))
        (elif (< (Variables|Default|GetActiveBigTargetCount) (Utilities|CeilingDivision (Variables|Default|GetMaxActiveTargetCount) 2))
          (goto _label_2)
          (else
            (goto _label)))))))

(fn TargetCleanup
  (params (SmallTarget :type BP%20Small%20Target%20Object%20Reference) (BigTarget :type BP%20Big%20Target%20Object%20Reference) (Small? :type Boolean))
  (if Small?
    (bind _result (Math|Integer|DecrementInt (Variables|Default|GetActiveSmallTargetCount))
      (:%20%20
        (if (== _result 0)
          (CallFunction|ActivateTarget true))
        (Utilities|Array|Add (Variables|Default|GetSmallTargets) SmallTarget)))
    (else
      (bind _result_2 (Math|Integer|DecrementInt (Variables|Default|GetActiveBigTargetCount))
        (:%20%20
          (if (== _result_2 0)
            (CallFunction|ActivateTarget false))
          (Utilities|Array|Add (Variables|Default|GetBigTargets) BigTarget))))))