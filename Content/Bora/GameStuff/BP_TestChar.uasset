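; Test pawn with free-flying movement that can pick up, trigger, drop and throw items.
; Hard-coded keys set axis values that Tick feeds into FloatingPawnMovement, with mouse look and a Shift speed boost, despite IMC_Default being added.
; A camera trace finds BPI_Item actors, which attach to a Scene component with physics off.
; Release or throw notifies BP_Item, detaches and restores physics, with throws adding velocity along the camera's forward vector.
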(event EventBeginPlay
  (bind _asplayer_controller (Utilities|Casting|CastToPlayerController (Pawn|GetController)))
  (Input|AddMappingContext (PlayerController|LocalPlayerSubsystems|GetEnhancedInputLocalPlayerSubsystem _asplayer_controller) "/Game/XRFramework/Input/IMC_Default.IMC_Default" 0 "(bIgnoreAllPressedKeysUntilRelease=True,bForceImmediately=False,bNotifyUserSettings=False)")
  (bind _asgm_xrgame_mode (Utilities|Casting|CastToGM_XRGameMode (Game|GetGameMode)))
  (Variables|Default|SetGMRef _asgm_xrgame_mode))

(event EventTick
  (params (DeltaSeconds :type Float%20%28single-precision%29))
  ;[0.15 0.15 0.15 0.5] Movement
  (Pawn|Input|AddMovementInput (Transformation|GetActorForwardVector) (Variables|Default|GetForwardInput) false)
  (Pawn|Input|AddMovementInput (Transformation|GetActorRightVector) (Variables|Default|GetRightInput) false)
  (Pawn|Input|AddMovementInput (Transformation|GetActorUpVector) (Variables|Default|GetUpInput) false))

(event Input|MouseEvents|MouseX
  (params (AxisValue :type Float%20%28single-precision%29))
  ;[0.15 0.15 0.15 0.5] Look Around
  (Pawn|Input|AddControllerYawInput AxisValue))

(event Input|MouseEvents|MouseY
  (params (AxisValue :type Float%20%28single-precision%29))
  ;[0.15 0.15 0.15 0.5] Look Around
  (Pawn|Input|AddControllerPitchInput (* AxisValue -1.0)))

(event Input|KeyboardEvents|W
  (params (Key :type Key%20Structure :default "None"))
  ;[0.15 0.15 0.15 0.5] Movement
  (:Pressed
    (Variables|Default|SetWHeld true)
    (Variables|Default|SetForwardInput 1.0))
  (:Released
    (Variables|Default|SetWHeld false)
    (if (Variables|Default|GetSHeld)
      (Variables|Default|SetForwardInput -1.0)
      (else
        (Variables|Default|SetForwardInput 0.0)))))

(event Input|KeyboardEvents|S
  (params (Key :type Key%20Structure :default "None"))
  ;[0.15 0.15 0.15 0.5] Movement
  (:Pressed
    (Variables|Default|SetSHeld true)
    (Variables|Default|SetForwardInput -1.0))
  (:Released
    (Variables|Default|SetSHeld false)
    (if (Variables|Default|GetWHeld)
      (Variables|Default|SetForwardInput 1.0)
      (else
        (Variables|Default|SetForwardInput 0.0)))))

(event Input|KeyboardEvents|F
  (params (Key :type Key%20Structure :default "None"))
  ;[0.15 0.15 0.15 0.5] Trigger Held Item
  (:Pressed
    (bind _helditem (Variables|Default|GetHeldItem)
      (:then
        (Class|BPIItem|Trigger(Message) _helditem))
      (:else))))

(event Input|KeyboardEvents|Tab
  (params (Key :type Key%20Structure :default "None"))
  ;[0.15 0.15 0.15 0.5] Cleanup
  (:Pressed
    (Variables|Default|SetHeldItem 0)
    (Variables|Default|SetItemHeld false)))

(event Input|KeyboardEvents|R
  (params (Key :type Key%20Structure :default "None"))
  ;[0.15 0.15 0.15 0.5] Pickup/Release Items
  (:Pressed
    (CallFunction|ThrowItem)))

(event Input|KeyboardEvents|A
  (params (Key :type Key%20Structure :default "None"))
  ;[0.15 0.15 0.15 0.5] Movement
  (:Pressed
    (Variables|Default|SetAHeld true)
    (Variables|Default|SetRightInput -1.0))
  (:Released
    (Variables|Default|SetAHeld false)
    (if (Variables|Default|GetDHeld)
      (Variables|Default|SetRightInput 1.0)
      (else
        (Variables|Default|SetRightInput 0.0)))))

(event Input|KeyboardEvents|D
  (params (Key :type Key%20Structure :default "None"))
  ;[0.15 0.15 0.15 0.5] Movement
  (:Pressed
    (Variables|Default|SetDHeld true)
    (Variables|Default|SetRightInput 1.0))
  (:Released
    (Variables|Default|SetDHeld false)
    (if (Variables|Default|GetAHeld)
      (Variables|Default|SetRightInput -1.0)
      (else
        (Variables|Default|SetRightInput 0.0)))))

(event Input|KeyboardEvents|Q
  (params (Key :type Key%20Structure :default "None"))
  ;[0.15 0.15 0.15 0.5] Movement
  (:Pressed
    (Variables|Default|SetUpInput -1.0))
  (:Released
    (Variables|Default|SetUpInput 0.0)))

(event Input|KeyboardEvents|E
  (params (Key :type Key%20Structure :default "None"))
  ;[0.15 0.15 0.15 0.5] Movement
  (:Pressed
    (Variables|Default|SetUpInput 1.0))
  (:Released
    (Variables|Default|SetUpInput 0.0)))

(event Input|KeyboardEvents|SpaceBar
  (params (Key :type Key%20Structure :default "None"))
  ;[0.15 0.15 0.15 0.5] Movement
  (:Pressed
    (Variables|Default|SetUpInput 1.0))
  (:Released
    (Variables|Default|SetUpInput 0.0)))

(event Input|KeyboardEvents|LeftCtrl
  (params (Key :type Key%20Structure :default "None"))
  ;[0.15 0.15 0.15 0.5] Movement
  (:Pressed
    (Variables|Default|SetUpInput -1.0))
  (:Released
    (Variables|Default|SetUpInput 0.0)))

(event Input|KeyboardEvents|LeftShift
  (params (Key :type Key%20Structure :default "None"))
  ;[0.15 0.15 0.15 0.5] Movement
  (:Pressed
    (Variables|/Script/Engine.FloatingPawnMovement|SetMaxSpeed (Variables|Default|GetFloatingPawnMovement) 2.4e+03))
  (:Released
    (Variables|/Script/Engine.FloatingPawnMovement|SetMaxSpeed (Variables|Default|GetFloatingPawnMovement) 1.2e+03)))

(event Input|KeyboardEvents|C
  (params (Key :type Key%20Structure :default "None"))
  (bind _camera (Variables|Default|GetCamera))
  (bind _returnvalue (Transformation|GetWorldLocation _camera))
  ;[0.15 0.15 0.15 0.5] Pickup/Release Items
  (:Pressed
    (if (not (Variables|Default|GetItemHeld))
      (bind _outhit (Collision|LineTraceByChannel _returnvalue (+ _returnvalue (* (Math|Vector|GetForwardVector _camera) 1e+03)) "TraceTypeQuery1" false 0 "None"))
      (if (Utilities|DoesObjectImplementInterface (.hitactor _outhit) "/Game/Bora/Blueprints/BPI_Item.BPI_Item_C")
        (CallFunction|EquipItem (.hitactor _outhit))
        (Variables|Default|SetItemHeld true))
      (else
        (CallFunction|ReleaseItem)))))

(fn ConstructionScript)

(fn EquipItem
  (params (Actor :type Actor%20Object%20Reference))
  (bind _scene (Variables|Default|GetScene))
  (bind _returnvalue (Transformation|GetWorldTransform _scene))
  (Physics|SetSimulatePhysics (Actor|GetComponentbyClass Actor "/Script/Engine.PrimitiveComponent") false)
  (Transformation|SetActorTransform Actor (Math|Transform|MakeTransform (.location _returnvalue) (.rotation _returnvalue) (Transformation|GetActorScale3D Actor)) false true)
  (Transformation|AttachComponentToComponent Actor (Variables|Default|GetScene) "None" "KeepWorld" "KeepWorld" "KeepWorld" true)
  (bind _output_get (Variables|Default|SetHeldItem Actor))
  (bind _asbp_item (Utilities|Casting|CastToBP_Item _output_get))
  (Default|Grabbed _asbp_item))

(fn ReleaseItem
  (bind _helditem (Variables|Default|GetHeldItem)
    (:then
      (bind _asbp_item (Utilities|Casting|CastToBP_Item _helditem))
      (Default|Released _asbp_item)
      (Transformation|DetachFromActor _helditem "KeepWorld" "KeepWorld" "KeepWorld")
      (Physics|SetSimulatePhysics (Actor|GetComponentbyClass _helditem "/Script/Engine.PrimitiveComponent") true)
      (Variables|Default|SetHeldItem 0)
      (Variables|Default|SetItemHeld false))
    (:else)))

(fn ThrowItem
  (bind _helditem (Variables|Default|GetHeldItem)
    (:then
      (bind _asbp_item (Utilities|Casting|CastToBP_Item _helditem))
      (Default|Released _asbp_item)
      (Transformation|DetachFromActor _helditem "KeepWorld" "KeepWorld" "KeepWorld")
      (Physics|SetSimulatePhysics (Actor|GetComponentbyClass _helditem "/Script/Engine.PrimitiveComponent") true)
      (Physics|SetPhysicsLinearVelocity (Actor|GetComponentbyClass _helditem "/Script/Engine.PrimitiveComponent") (* (Math|Vector|GetForwardVector (Variables|Default|GetCamera)) (Variables|Default|GetThrowStrength)) true "None")
      (Variables|Default|SetHeldItem 0)
      (Variables|Default|SetItemHeld false))
    (:else)))